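; Game instance that handles saving and loading the player's position and tracks unlocked doors by name.
; SaveGame asynchronously writes the pawn's location, rotation and map name to a single fixed MySaveGame slot.
; LoadGame reads that slot, requests the saved level if different, then immediately sets the pawn's transform without waiting for the level change.
; UnlockDoor and IsDoorUnlocked manage the UnlockedDoors list, which is not written to the save.
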(event Custom|Load%20Game
  ;[1 1 1] Load from harddrive
  (bind (_savegame _bsuccess) (|AsyncLoadGamefromSlot "Slot 1")
    (:Completed
      (if _bsuccess
        (bind _asmy_save_game (Utilities|Casting|CastToMySaveGame _savegame))
        (bind _returnvalue (Game|GetCurrentLevelName true))
        (if (Utilities|Enum|Equal(Enum) _returnvalue (Utilities|String|ToString(Name) (Variables|/Game/Blueprints/GameInstancesAndSaves/MySaveGame.MySaveGame_C|GetmapName _asmy_save_game)))
          _
          (else
            ;[1 1 1] Update data
            (Game|OpenLevel(byName) (Variables|/Game/Blueprints/GameInstancesAndSaves/MySaveGame.MySaveGame_C|GetmapName _asmy_save_game))))
        (Transformation|SetActorLocationAndRotation (Game|Player|GetPlayerPawn 0) (Variables|/Game/Blueprints/GameInstancesAndSaves/MySaveGame.MySaveGame_C|GetplayerLocation _asmy_save_game) (Variables|/Game/Blueprints/GameInstancesAndSaves/MySaveGame.MySaveGame_C|GetplayerRotation _asmy_save_game))))))

(event Custom|Save%20Game
  (bind _returnvalue (Game|Player|GetPlayerPawn 0))
  ;[1 1 1] instantiate save game object
  (bind _returnvalue_2 (SaveGame|CreateSaveGameObject "/Game/Blueprints/GameInstancesAndSaves/MySaveGame.MySaveGame_C")) ; what we set up in the save game is saved
  ;[1 1 1] populate the data
  (Variables|/Game/Blueprints/GameInstancesAndSaves/MySaveGame.MySaveGame_C|SetplayerLocation _returnvalue_2 (Transformation|GetActorLocation _returnvalue))
  (Variables|/Game/Blueprints/GameInstancesAndSaves/MySaveGame.MySaveGame_C|SetplayerRotation _returnvalue_2 (Transformation|GetActorRotation _returnvalue))
  (bind _returnvalue_3 (Game|GetCurrentLevelName true))
  (Variables|/Game/Blueprints/GameInstancesAndSaves/MySaveGame.MySaveGame_C|SetmapName _returnvalue_2 (Utilities|String|StringToName _returnvalue_3))
  ;[1 1 1] Save to hard drive
  (bind _bsuccess (|AsyncSaveGametoSlot _returnvalue_2 "Slot 1")
    (:Completed
      ;[1 1 1] Feedback
      (if _bsuccess
        (Development|PrintString "Save successful")
        (else
          (Development|PrintString "Save failed"))))))

(fn IsDoorUnlocked
  (params (door%20name :type String))
  (return (Utilities|Array|ContainsItem (Variables|Default|GetUnlockedDoors) door%20name)))

(fn UnlockDoor
  (params (door%20name :type String))
  (Utilities|Array|AddUnique (Variables|Default|GetUnlockedDoors) door%20name))