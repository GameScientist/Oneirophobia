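; Grey weaver enemy that clings to ceilings, drops when it detects TobyGuy below and damages him by falling impact or bite.
; Tick maintains ceiling cling through upward impulses and runs an Idle/Aggro/Attack state switch.
; Idle traces find ceiling and player, Flip swaps flying and falling, and Aggro restores walking on landing.
; In Attack, a timeline rotates the biters and toggles hitbox overlaps, then returns to Aggro.
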(event OnComponentBeginOverlap(HitBox)
  (params (OverlappedComponent :type Primitive%20Component%20Object%20Reference) (OtherActor :type Actor%20Object%20Reference) (OtherComp :type Primitive%20Component%20Object%20Reference) (OtherBodyIndex :type Integer) (bFromSweep :type Boolean) (SweepResult :type Hit%20Result%20Structure%20%28by%20ref%29))
  ;[1 1 1] Applies damage to the if the player is within range of the grey weaver's attack.
  (bind _astoby_guy (Utilities|Casting|CastToTobyGuy OtherActor))
  (Game|Damage|ApplyDamage _astoby_guy 1.0 0 0)
  (Development|PrintString "Ow!"))

(event EventTick
  (params (DeltaSeconds :type Float%20%28single-precision%29))
  (bind _hitbox (Variables|Default|GetHitBox))
  (|CallParentFunction DeltaSeconds)
  (Utilities|IsValid self
    (:Is%20Valid
      (Utilities|FlowControl|Sequence
        (:then_0
          (CallFunction|CeilingStatus))
        (:then_1
          ;[1 1 1] State Handling
          (switch Utilities|FlowControl|Switch|SwitchonEnemyState (Variables|Default|Getstate)
            (:NewEnumerator0
              (CallFunction|LookDown))
            (:NewEnumerator1
              (CallFunction|CheckforLanding))
            (:NewEnumerator2
              (Utilities|FlowControl|DoOnce false :!label _label
                (:Completed
                  (bind (_direction _biter1 _biter2) (Timeline|Bite PlayFromStart)
                    (:Update
                      (CallFunction|BiteMovement _biter1 _biter2))
                    (:Finished
                      (Variables|Default|Setstate "NewEnumerator1")
                      (goto _label Reset))
                    (:EnableHitBox
                      (Variables|/Script/Engine.PrimitiveComponent|SetbGenerateOverlapEvents _hitbox true))
                    (:Disable%20Hit%20Box
                      (Variables|/Script/Engine.PrimitiveComponent|SetbGenerateOverlapEvents _hitbox false))))))))))))

(event Collision|EventHit
  (params (MyComp :type Primitive%20Component%20Object%20Reference) (Other :type Actor%20Object%20Reference) (OtherComp :type Primitive%20Component%20Object%20Reference) (bSelfMoved :type Boolean) (HitLocation :type Vector :default "0, 0, 0") (HitNormal :type Vector :default "0, 0, 0") (NormalImpulse :type Vector :default "0, 0, 0") (Hit :type Hit%20Result%20Structure%20%28by%20ref%29))
  ;[1 1 1] The grey weaver damages the player when falling from the ceiling.
  (bind _astoby_guy (Utilities|Casting|CastToTobyGuy (.HitActor (Collision|BreakHitResult Hit))))
  (if (AI|Components|NavMovement|IsFalling (Variables|Character|GetCharacterMovement))
    (Game|Damage|ApplyDamage _astoby_guy 1.0 0 0)))

(fn ConstructionScript
  (|CallParentFunction)
  (Variables|Default|SetmoveToAcceptanceRadius 1e+02))

(fn Flip
  (params (NewMovementMode :type EMovementMode%20Enum :default "MOVE_None") (New%20Rotation%20X%20%28Roll%29 :type Float%20%28single-precision%29) (onCeiling :type Boolean))
  (Pawn|Components|CharacterMovement|SetMovementMode (Variables|Character|GetCharacterMovement) NewMovementMode 0)
  (Transformation|SetRelativeRotation (Variables|Default|GetSphere) (Math|Rotator|MakeRotator New%20Rotation%20X%20%28Roll%29 0.0 0.0) false false)
  (Variables|Default|SetonCeiling onCeiling))

(fn ClingtoCeiling
  (CallFunction|Flip "MOVE_Flying" 1.8e+02 true)
  (Variables|Default|SetinAir true))

(fn VerticalLookResult
  (params (LookTarget :type Float%20%28single-precision%29) (lookingUp :type Boolean))
  (bind (_startpoint _endpoint) (CallFunction|TraceStartandEndPoints LookTarget))
  (if lookingUp
    ;[1 1 1] Look Up
    (bind _outhit (Collision|SphereTraceByChannel _startpoint _endpoint 5e+01 "TraceTypeQuery1" false 0 "ForOneFrame"))
    (else
      ;[1 1 1] Look Down
      (bind _outhit_2 (Collision|BoxTraceByChannel _startpoint _endpoint "200.000000,200.000000,1.000000" "0, 0, 0" "TraceTypeQuery2" false 0 "ForOneFrame"))))
  (return (.bBlockingHit (Collision|BreakHitResult _outhit)) (.HitActor (Collision|BreakHitResult _outhit_2))))

(fn LookUp
  (if (Utilities|Enum|Equal(Enum) (Variables|Default|Getstate) "NewEnumerator0")
    (bind _bblockinghit (CallFunction|VerticalLookResult 5e+02 true))
    (if _bblockinghit
      (CallFunction|ClingtoCeiling)
      (else
        (Transformation|SetActorLocation (Variables|Default|GetidleLocation) false true)))))

(fn CeilingStatus
  (if (Variables|Default|GetonCeiling)
    (Physics|AddImpulse (Variables|Character|GetCharacterMovement) "0.000000, 0,1000.000000" true)
    (else
      (CallFunction|LookUp))))

(fn LookDown
  (bind _hitactor (CallFunction|VerticalLookResult -5e+02 false))
  (Utilities|Casting|CastToTobyGuy _hitactor)
  (Variables|Default|Setstate "NewEnumerator1")
  (CallFunction|Flip "MOVE_Falling" 0.0 false))

(fn CheckforLanding
  (bind _returnvalue (CallFunction|HasLanded))
  (if _returnvalue
    (Pawn|Components|CharacterMovement|SetMovementMode (Variables|Character|GetCharacterMovement) "MOVE_Walking" 0)))

(fn BiteMovement
  (params (NewRotation_Yaw :type Float%20%28single-precision%29) (NewRotation_Yaw2 :type Float%20%28single-precision%29))
  (Transformation|SetRelativeRotation (Variables|Default|GetBiterRotator1) (Math|Rotator|MakeRotator 0.0 0.0 NewRotation_Yaw) false false)
  (Transformation|SetRelativeRotation (Variables|Default|GetBiterRotator2) (Math|Rotator|MakeRotator 0.0 0.0 NewRotation_Yaw2) false false))

(fn TraceStartandEndPoints
  (params (Distance :type Float%20%28single-precision%29))
  (bind _returnvalue (Transformation|GetActorLocation))
  (return _returnvalue (+ _returnvalue (* (Math|Vector|GetUpVector (Transformation|GetWorldRotation (Variables|Default|GetCapsuleComponent))) Distance))))

(fn HasLanded
  (bind _charactermovement (Variables|Character|GetCharacterMovement))
  (return (and (AI|Components|NavMovement|IsFalling _charactermovement) (.bWalkableFloor (Utilities|Struct|BreakFindFloorResult (Pawn|Components|CharacterMovement|FindFloor _charactermovement (Transformation|GetWorldLocation (Variables|Default|GetCapsuleComponent))))))))