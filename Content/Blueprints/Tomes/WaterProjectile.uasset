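; Water tome projectile that damages enemies it passes through.
; On sphere overlap with an EnemyBaseCharacter, it spawns an impact effect at the enemy and applies damage without destroying itself.
; It remembers only the last enemy hit to skip back-to-back repeat hits on the same target.
; Overlapping any non-enemy or registering a blocking hit on the sphere destroys it.
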(event OnComponentBeginOverlap(Sphere)
  (params (OverlappedComponent :type Primitive%20Component%20Object%20Reference) (OtherActor :type Actor%20Object%20Reference) (OtherComp :type Primitive%20Component%20Object%20Reference) (OtherBodyIndex :type Integer) (bFromSweep :type Boolean) (SweepResult :type Hit%20Result%20Structure%20%28by%20ref%29))
  (bind _asenemy_base_character (Utilities|Casting|CastToEnemyBaseCharacter OtherActor)
    (:then
      (if (!= (Variables|Default|GetLastHit) OtherActor)
        (Niagara|SpawnSystematLocation "/Game/Art/Particles/DonovanF_Particles/FX_WaterProjectile_Impact.FX_WaterProjectile_Impact" (Transformation|GetActorLocation _asenemy_base_character))
        (Game|Damage|ApplyDamage OtherActor (Variables|Default|GetDamage) 0 0)
        (Variables|Default|SetLastHit OtherActor)))
    (:CastFailed
      (Actor|DestroyActor))))

(event OnComponentHit(Sphere)
  (params (HitComponent :type Primitive%20Component%20Object%20Reference) (OtherActor :type Actor%20Object%20Reference) (OtherComp :type Primitive%20Component%20Object%20Reference) (NormalImpulse :type Vector :default "0, 0, 0") (Hit :type Hit%20Result%20Structure%20%28by%20ref%29))
  (Actor|DestroyActor))

(fn ConstructionScript
  (|CallParentFunction))