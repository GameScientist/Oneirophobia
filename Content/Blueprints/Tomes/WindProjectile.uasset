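; Wind tome projectile that damages and knocks back enemies on contact.
; On sphere overlap it applies damage to any actor, pushes EnemyBaseCharacter targets along the Scene component's forward vector, then destroys itself; blocking hits just destroy it.
; Overlap and hit spawn a non-auto-destroying ForceBurst effect without a set location, and the Destroyed event spawns another at the sphere's position.
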(event OnComponentBeginOverlap(Sphere)
  (params (OverlappedComponent :type Primitive%20Component%20Object%20Reference) (OtherActor :type Actor%20Object%20Reference) (OtherComp :type Primitive%20Component%20Object%20Reference) (OtherBodyIndex :type Integer) (bFromSweep :type Boolean) (SweepResult :type Hit%20Result%20Structure%20%28by%20ref%29))
  (Game|Damage|ApplyDamage OtherActor (Variables|Default|GetDamage) 0 0)
  (bind _asenemy_base_character (Utilities|Casting|CastToEnemyBaseCharacter OtherActor)
    (:then
      (Default|KnockBack _asenemy_base_character (Math|Vector|GetForwardVector (Variables|Default|GetScene))))
    (:CastFailed
      _))
  (Niagara|SpawnSystematLocation "/Game/Art/Particles/Force/ForceBurst.ForceBurst" "0, 0, 0" "0, 0, 0" "1.000000,1.000000,1.000000" false)
  (Actor|DestroyActor))

(event OnComponentHit(Sphere)
  (params (HitComponent :type Primitive%20Component%20Object%20Reference) (OtherActor :type Actor%20Object%20Reference) (OtherComp :type Primitive%20Component%20Object%20Reference) (NormalImpulse :type Vector :default "0, 0, 0") (Hit :type Hit%20Result%20Structure%20%28by%20ref%29))
  (Niagara|SpawnSystematLocation "/Game/Art/Particles/Force/ForceBurst.ForceBurst" "0, 0, 0" "0, 0, 0" "1.000000,1.000000,1.000000" false)
  (Actor|DestroyActor))

(event EventDestroyed
  (Niagara|SpawnSystematLocation "/Game/Art/Particles/Force/ForceBurst.ForceBurst" (Transformation|GetWorldLocation (Variables|Default|GetSphere))))

(event EventTick
  (params (DeltaSeconds :type Float%20%28single-precision%29))
  (|CallParentFunction DeltaSeconds))

(fn ConstructionScript
  (|CallParentFunction))