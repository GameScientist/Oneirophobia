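; BaseProjectile is a projectile actor under Tomes that spawns a shot particle effect on BeginPlay and flies until its lifetime expires.
; Tick moves the Scene component manually along its forward vector by Velocity, without sweep or a movement component.
; Gravity adds a per-frame Z drop that grows with accumulated time but is not scaled by delta time.
; LifeTime drains at three times real time, and the graph contains no hit or damage logic.
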(event EventTick
  (params (DeltaSeconds :type Float%20%28single-precision%29))
  (bind _velocity (Variables|Default|GetVelocity))
  (bind _scene (Variables|Default|GetScene))
  (bind _scene_2 (Variables|Default|GetScene))
  (bind _returnvalue (Math|Vector|GetForwardVector _scene))
  (bind _returnvalue_2 (* _returnvalue DeltaSeconds))
  (bind _returnvalue_3 (* _returnvalue_2 _velocity))
  ;[1 1 1] Moves Projectiles
  (Variables|Default|SetDtBeingAddedUp (+ DeltaSeconds (Variables|Default|GetDtBeingAddedUp)))
  (Transformation|SetWorldLocation _scene_2 (+ (Math|Vector|MakeVector (.x _returnvalue_3) (.y _returnvalue_3) (- (.z _returnvalue_3) (* (Variables|Default|GetDtBeingAddedUp) (Variables|Default|GetGravity)))) (Transformation|GetWorldLocation _scene_2)) false false)
  ;[1 1 1] Trakcs LifeTime and destroys if it reaches 0
  (bind _output_get (Variables|Default|SetLifeTime (- (Variables|Default|GetLifeTime) (* 3 DeltaSeconds))))
  (if (<= _output_get 0.0)
    (Actor|DestroyActor)))

(event EventBeginPlay
  (Niagara|SpawnSystematLocation (Variables|Default|GetShotParticleEffect) (Transformation|GetActorLocation) (Transformation|GetActorRotation)))

(fn ConstructionScript)